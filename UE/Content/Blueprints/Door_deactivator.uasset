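; Door deactivator actor that briefly removes collision from a referenced Door's static mesh when the player character overlaps it.
; Begin overlap disables the mesh collision and sets an Open flag.
; Tick clears that flag on its next pass, then restores QueryAndPhysics collision on every pass where it is false, so the door stays passable only momentarily rather than for the whole overlap.
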(event `self.ReceiveBeginPlay`
  (set `self.Open` false))

(event `self.ReceiveActorBeginOverlap`
  (params (OtherActor :type "Actor Object Reference"))
  (if (== (`GameplayStatics.GetPlayerCharacter` 0) OtherActor)
    (`PrimitiveComponent.SetCollisionEnabled` (`StaticMeshActor.StaticMeshComponent` (`self.Door`)) "NoCollision")
    (set `self.Open` true)))

(event `self.ReceiveTick`
  (params (DeltaSeconds :type "Float (single-precision)"))
  (if (`self.Open`)
    (set `self.Open` false)
    (else
      (`PrimitiveComponent.SetCollisionEnabled` (`StaticMeshActor.StaticMeshComponent` (`self.Door`)) "QueryAndPhysics"))))

(fn `UserConstructionScript`)